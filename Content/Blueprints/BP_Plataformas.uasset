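; Moving platform that travels through an array of waypoint actors, PuntosDePlataforma, and loops back to the first.
; Each tick, VInterpTo eases it toward the current point at rate Velocidad, without sweeping, resetting Index to zero when it is invalid.
; Its Box overlapping any actor tagged "Punto" advances Index, unless the current and next entries are identical, and prints a debug string.
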(event `self.ReceiveTick`
  (params (DeltaSeconds :type "Float (single-precision)"))
  (`self.Movimiento`))

(event `Movimiento`
  (bind _puntosdeplataforma (`self.PuntosDePlataforma`))
  (if (`KismetArrayLibrary.Array_IsValidIndex` _puntosdeplataforma (`self.Index`))
    (`self.K2_SetActorLocation` (`KismetMathLibrary.VInterpTo` (`self.K2_GetActorLocation`) (`self.K2_GetActorLocation` (`|GetArrayItem` _puntosdeplataforma (`self.Index`))) (`GameplayStatics.GetWorldDeltaSeconds`) (`self.Velocidad`)))
    (else
      (set `self.Index` 0))))

(event `self.Box.OnComponentBeginOverlap`
  (params (OverlappedComponent :type "PrimitiveComponent Object Reference") (OtherActor :type "Actor Object Reference") (OtherComp :type "PrimitiveComponent Object Reference") (OtherBodyIndex :type Integer) (bFromSweep :type Boolean) (SweepResult :type "HitResult Structure (by ref)"))
  (if (and (`self.ActorHasTag` OtherActor "Punto") (not (== (`|GetArrayItem` (`self.PuntosDePlataforma`) (`self.Index`)) (`|GetArrayItem` (`self.PuntosDePlataforma`) (+ (`self.Index`) 1)))))
    (`/Engine/EditorBlueprintResources/StandardMacros.IncrementInt` (`self.Index`)
      (:`  `
        (`KismetSystemLibrary.PrintString` "Hello")))))

(fn `UserConstructionScript`)